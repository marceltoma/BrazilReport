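; Clickable map actor for one state, with name, UF and region group, that highlights on mouse hover and can be marked selected through custom depth.
; Mesh cursor and click events fire dispatchers on ReportGameState, which every state binds to for updating its highlight.
; UserLevel 0 lights the hovered state's whole region, while level 1 lights only that state within the selected region.
; Highlights recolor a dynamic material instance created in the construction script.
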(event OnClicked(MeshEstado)
  (params (TouchedComponent :type Primitive%20Component%20Object%20Reference))
  ;[1 1 1] Quando clicar, chama o evento ClicouMouse do gamestate, tem um bind nesse evento no Blueprint Level
  (Development|PrintString (Utilities|String|ToString(Text) (Utilities|Text|FormatText "{state}/{UF} - {Region}" (Utilities|Text|ToText(String) (Variables|Default|GetStateName)) (Utilities|Text|ToText(String) (Variables|Default|GetUF)) (Utilities|Text|ToText(String) (Variables|Default|GetRegionGroup)))))
  (bind _asreport_game_state (Utilities|Casting|CastToReportGameState (Game|GetGameState)))
  (Default|CallClicouMouse _asreport_game_state self)
  (Default|CallSaiuMouse _asreport_game_state)
  (Default|CallPassouMouse _asreport_game_state))

(event OnBeginCursorOver(MeshEstado)
  (params (TouchedComponent :type Primitive%20Component%20Object%20Reference))
  ;[1 1 1] Call custom event
  (bind _asreport_game_state (Utilities|Casting|CastToReportGameState (Game|GetGameState)))
  (Variables|/Game/Blueprints/ReportGameState.ReportGameState_C|SetSelectedState _asreport_game_state self)
  (Default|CallPassouMouse _asreport_game_state))

(event OnEndCursorOver(MeshEstado)
  (params (TouchedComponent :type Primitive%20Component%20Object%20Reference))
  ;[1 1 1] Call custom event
  (bind _asreport_game_state (Utilities|Casting|CastToReportGameState (Game|GetGameState)))
  (Default|CallSaiuMouse _asreport_game_state))

(event Custom|BeginCursorOver
  ;[1 1 1] Efetua logica de highlight do mouseOver
  (bind _asreport_game_state (Utilities|Casting|CastToReportGameState (Game|GetGameState)))
  (switch int (Variables|/Game/Blueprints/ReportGameState.ReportGameState_C|GetUserLevel _asreport_game_state)
    (:0
      (if (Utilities|Enum|Equal(Enum) (Variables|State_C|GetRegionGroup (Variables|/Game/Blueprints/ReportGameState.ReportGameState_C|GetSelectedState _asreport_game_state)) (Variables|Default|GetRegionGroup))
        (Rendering|Material|SetVectorParameterValue (Variables|Default|GetparamMatEstado) "CorPadrao" (Variables|Default|GetStateColorOver) :!class /Script/Engine.MaterialInstanceDynamic :!label _label)
        (Rendering|Material|SetVectorParameterValue (Variables|Default|GetparamMatEstado) "EmissiveColor" (Variables|Default|GetStateColorOver) :!class /Script/Engine.MaterialInstanceDynamic)))
    (:1
      ;;[1 1 1] Lógica de highlight para regiao
      (if (and (Utilities|Enum|Equal(Enum) (Variables|/Game/Blueprints/ReportGameState.ReportGameState_C|GetselectedRegion _asreport_game_state) (Variables|Default|GetRegionGroup)) (Utilities|Enum|Equal(Enum) (Variables|State_C|GetStateName (Variables|/Game/Blueprints/ReportGameState.ReportGameState_C|GetSelectedState _asreport_game_state)) (Variables|Default|GetStateName)))
        (goto _label)))))

(event Custom|EndCursorOver
  ;[1 1 1] Volta ao estado anterior quando tirar o mouse
  (Rendering|Material|SetVectorParameterValue (Variables|Default|GetparamMatEstado) "CorPadrao" (Variables|Default|GetStateColor) :!class /Script/Engine.MaterialInstanceDynamic)
  (Rendering|Material|SetVectorParameterValue :self (Variables|Default|GetparamMatEstado) :ParameterName "EmissiveColor" :!class /Script/Engine.MaterialInstanceDynamic))

(event EventBeginPlay
  ;[1 1 1] Binding event dispatchers
  (bind _asreport_game_state (Utilities|Casting|CastToReportGameState (Game|GetGameState)))
  (EventDispatchers|BindEventtoPassouMouse _asreport_game_state (delegate Custom|BeginCursorOver))
  (EventDispatchers|BindEventtoSaiuMouse _asreport_game_state (delegate Custom|EndCursorOver)))

(fn ConstructionScript
  (Components|StaticMesh|SetStaticMesh (Variables|Default|GetparamMeshEstado))
  (bind _returnvalue (Rendering|Material|CreateDynamicMaterialInstance "/Game/Materials/StateMat.StateMat" :!class /Script/Engine.KismetMaterialLibrary))
  (bind _output_get (Variables|Default|SetparamMatEstado _returnvalue))
  (Rendering|Material|SetVectorParameterValue _output_get "CorPadrao" (Variables|Default|GetStateColor) :!class /Script/Engine.MaterialInstanceDynamic)
  (Rendering|Material|SetMaterial 0 _output_get))

(fn Selecionar
  (Rendering|SetRenderCustomDepth (Variables|Default|GetMeshEstado) true)
  (bind _output_get (Variables|Default|SetisSelected true))
  (return _output_get))

(fn Deselecionar
  (Rendering|SetRenderCustomDepth (Variables|Default|GetMeshEstado) false)
  (Variables|Default|SetisSelected false)
  (return false))